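; Player throw attack actor that deals the player's damage to enemies and destroys itself on a hit or three seconds after spawning.
; Sphere overlap casts to blob enemy and, if its Hit flag is set, calls DmgBadMan.
; The skeleton check sits behind a successful blob cast with Hit false, so skeletons alone never reach it.
; BeginPlay caches tagged tree, skeleton and blob enemies, but the overlap ignores them.
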(event OnComponentBeginOverlap(Sphere)
  (params (OverlappedComponent :type Primitive%20Component%20Object%20Reference) (OtherActor :type Actor%20Object%20Reference) (OtherComp :type Primitive%20Component%20Object%20Reference) (OtherBodyIndex :type Integer) (bFromSweep :type Boolean) (SweepResult :type Hit%20Result%20Structure%20%28by%20ref%29))
  (bind _asblob_enemy (Utilities|Casting|CastToblob_enemy OtherActor))
  (if (Variables|/Game/Enemy/blob_enemy.blob_enemy_C|GetHit _asblob_enemy)
    (bind _asblob_enemy_2 (Utilities|Casting|CastToblob_enemy OtherActor))
    (bind _asplayer_bp (Utilities|Casting|CastToPlayer_BP (Game|GetPlayerCharacter 0)))
    (Default|DmgBadMan _asblob_enemy_2 (Variables|/Game/Player/Player_BP.Player_BP_C|Getdamage _asplayer_bp))
    (Development|PrintString "Hit Blob")
    (Actor|DestroyActor)
    (else
      (bind _asenemy (Utilities|Casting|CastToskel_enemy OtherActor))
      (if (Variables|/Game/Enemy/skel_enemy.skel_enemy_C|GetHit _asenemy)
        (bind _asenemy_2 (Utilities|Casting|CastToskel_enemy OtherActor))
        (bind _asplayer_bp_2 (Utilities|Casting|CastToPlayer_BP (Game|GetPlayerCharacter 0)))
        (Default|DmgBadMan _asenemy_2 (Variables|/Game/Player/Player_BP.Player_BP_C|Getdamage _asplayer_bp_2))
        (Development|PrintString "Hit Skeleton")
        (Actor|DestroyActor)))))

(event EventBeginPlay
  (bind _outactors (Actor|GetAllActorswithTag "TreeEnemy"))
  (Variables|Default|SetTreeEnemy (Utilities|Array|Get(acopy) _outactors))
  (bind _outactors_2 (Actor|GetAllActorswithTag "SkeletonEnemy"))
  (Variables|Default|SetSkeletonEnemy (Utilities|Array|Get(acopy) _outactors_2))
  (bind _outactors_3 (Actor|GetAllActorswithTag "BlobEnemy"))
  (Variables|Default|SetBlobEnemy (Utilities|Array|Get(acopy) _outactors_3))
  (Utilities|FlowControl|Delay 3.0)
  (Actor|DestroyActor))

(fn ConstructionScript)