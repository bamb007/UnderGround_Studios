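; Player character for a 2D side-scroller, with movement, energy-costing jumps, wall jumps and a right-click thrown attack.
; Tick regenerates energy after a delay, turns the character toward its travel direction and selects a flipbook through a branch-based state function.
; Airborne jumps line-trace for walls and launch away on a hit.
; Attack-flag setters and the wall-jump limit are unwired, and falling/jumping flags enter the animation function swapped.
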(event Custom|UpdateAnimation
  (bind _returnvalue (Transformation|GetVelocity))
  (bind (_x _y _z) (Math|Vector|BreakVector _returnvalue))
  ;[1 1 1] UpdateAnimation
  (Variables|Default|SetisMoveing (!= _x 0.0))
  (Variables|Default|SetisFalling (< _z 0.0))
  (Variables|Default|SetisJumping (> _z 0.1))
  (bind _flipbook (CallFunction|AnimationStateMachine (Variables|Default|GetisJumping) (Variables|Default|GetisMoveing) (Variables|Default|GetisAttacking) (Variables|Default|GetisThrowing) (Variables|Default|GetisFalling)))
  (Sprite|SetFlipbook (Variables|Default|GetSprite) _flipbook))

(event Custom|EnergyRegen
  ;[1 1 1] EnergyRegen
  (if (< (Variables|Default|Getenergy) (Variables|Default|GetmaxEnergy))
    (Utilities|FlowControl|Delay 0.2)
    (Variables|Default|Setenergy (+ (Variables|Default|Getenergy) (Variables|Default|GetenergyRegenPS)))
    (if (> (Variables|Default|Getenergy) (Variables|Default|GetmaxEnergy))
      (Variables|Default|Setenergy (Variables|Default|GetmaxEnergy)))))

(event Custom|WallJump
  (bind _returnvalue (Transformation|GetActorLocation))
  (bind _returnvalue_2 (Transformation|GetActorForwardVector))
  (bind _capsulecomponent (Variables|Collision|GetCapsuleComponent))
  (bind _returnvalue_3 (Components|Capsule|GetScaledCapsuleRadius _capsulecomponent))
  (bind _returnvalue_4 (+ _returnvalue_3 15.0))
  ;[1 1 1] WallJump
  (bind (_outhit _returnvalue_5) (Collision|LineTraceByChannel (- _returnvalue (* _returnvalue_2 _returnvalue_4)) (+ _returnvalue (* _returnvalue_2 _returnvalue_4)) "TraceTypeQuery1" true 0 "None"))
  (if _returnvalue_5
    (Character|LaunchCharacter (Math|Vector|MakeVector (* (Math|Float|Sign(Float) (- (.x (Transformation|GetActorLocation)) (.x (.Location (Collision|BreakHitResult _outhit))))) 4.5e+02) 0.0 (Variables|/Script/Engine.CharacterMovementComponent|GetJumpZVelocity (Variables|Character|GetCharacterMovement))) true true)
    (elif (< (Variables|Default|GetjumpCounter) (Variables|Default|GetJumpMaxCount))
      (Character|Jump))))

(event EventOnLanded
  (params (Hit :type Hit%20Result%20Structure%20%28by%20ref%29))
  ;[1 1 1] Handle Jump
  ;;[1 1 1] Checks if the player is grounded
  (Variables|Default|SetGrounded true)
  (Variables|Default|SetjumpCounter 0)
  (Variables|Default|SetwallJumpCounter 0))

(event EventTick
  (params (DeltaSeconds :type Float%20%28single-precision%29))
  ;[1 1 1] EventTick (UpdateAnimation / energyRegen)
  (CallFunction|EnergyRegen)
  (CallFunction|UpdateAnimation)
  (Math|Float|CompareFloat (.X (Math|Vector|BreakVector (Variables|/Script/Engine.MovementComponent|GetVelocity (Pawn|GetMovementComponent)))) 0.0
    (:>
      (Pawn|SetControlRotation (Pawn|GetController) (Math|Rotator|MakeRotator 0.0 0.0 0.0) :!label _label))
    (:==
      (if (Variables|Default|GetmoveingRight)
        (goto _label)
        (else
          (Pawn|SetControlRotation (Pawn|GetController) (Math|Rotator|MakeRotator 0.0 0.0 1.8e+02) :!label _label_2))))
    (:<
      (goto _label_2))))

(event EventBeginPlay
  ;[1 1 1] BeginPlay
  ;;[1 1 1] SetValues
  (Variables|Default|SetGrounded true)
  (Variables|Default|Setenergy (Variables|Default|GetmaxEnergy))
  (Variables|Default|Sethealth (Variables|Default|GetmaxHealth)))

(event EventOnJumped
  ;[1 1 1] Handle Jump
  ;;[1 1 1] Checks when the player is not grounded
  (Variables|Default|SetGrounded false))

(event Input|ActionEvents|InputActionJump
  (params (Key :type Key%20Structure))
  (bind _jumpcost (Variables|Default|GetjumpCost))
  ;[1 1 1] Handle Jump
  (:Pressed
    (if (< (Variables|Default|GetjumpCounter) (Variables|Default|GetJumpMaxCount))
      (if (>= (Variables|Default|Getenergy) _jumpcost)
        (Variables|Default|Setenergy (- (Variables|Default|Getenergy) _jumpcost))
        (if (Variables|Default|Getgrounded)
          (Character|Jump)
          ;;[1 1 1] Connect in branch middle to add walljump to jumpcounter
          (Variables|Default|SetjumpCounter (+ (Variables|Default|GetjumpCounter) 1))
          (else
            (CallFunction|WallJump))))))
  (:Released
    (Character|StopJumping)))

(event Input|AxisEvents|InputAxisMove
  (params (AxisValue :type Float%20%28single-precision%29))
  ;[1 1 1] Movement
  (if (> AxisValue 0.0)
    (Variables|Default|SetmoveingRight true)
    (elif (< AxisValue 0.0)
      (Variables|Default|SetmoveingRight false)))
  (Pawn|Input|AddMovementInput "1.000000,0.000000, 0" AxisValue false))

(event Input|KeyboardEvents|Escape
  (params (Key :type Key%20Structure))
  ;[1 1 1] FastExitGame
  (:Pressed
    (Development|ExecuteConsoleCommand "EXIT")))

(event Input|MouseEvents|LeftMouseButton
  (params (Key :type Key%20Structure))
  ;[1 1 1] TestArea
)

(event Input|MouseEvents|RightMouseButton
  (params (Key :type Key%20Structure))
  ;[1 1 1] TestArea
  (:Pressed
    (Game|SpawnActorfromClass "/Game/Player/PlayerAttack/ThrowAttack_BP.ThrowAttack_BP_C" (Transformation|GetWorldTransform (Variables|Default|GetShootingPoint)) "Undefined" 0 0)))

(event Input|TouchEvents|InputTouch
  (params (Location :type Vector) (FingerIndex :type ETouchIndex%20Enum))
  (bind _jumpcost (Variables|Default|GetjumpCost))
  ;[1 1 1] Handle Jump
  (:Pressed
    (if (< (Variables|Default|GetjumpCounter) (Variables|Default|GetJumpMaxCount))
      (if (>= (Variables|Default|Getenergy) _jumpcost)
        (Variables|Default|Setenergy (- (Variables|Default|Getenergy) _jumpcost))
        (if (Variables|Default|Getgrounded)
          (Character|Jump)
          ;;[1 1 1] Connect in branch middle to add walljump to jumpcounter
          (Variables|Default|SetjumpCounter (+ (Variables|Default|GetjumpCounter) 1))
          (else
            (CallFunction|WallJump))))))
  (:Released
    (Character|StopJumping)))

(fn ConstructionScript)

(fn AnimationStateMachine
  (params (isFalling :type Boolean) (isMoveing :type Boolean) (isAttacking :type Boolean) (isThrowing :type Boolean) (isJumping :type Boolean))
  (if isFalling
    (LocalVariables|SetAnimationState "NewEnumerator3")
    (elif isMoveing
      (LocalVariables|SetAnimationState "NewEnumerator2")
      (elif isAttacking
        (LocalVariables|SetAnimationState "NewEnumerator4")
        (elif isThrowing
          (LocalVariables|SetAnimationState "NewEnumerator5")
          (elif isJumping
            (LocalVariables|SetAnimationState "NewEnumerator1")
            (else
              (LocalVariables|SetAnimationState "NewEnumerator0")))))))
  (return (Utilities|Select :Index (LocalVariables|GetAnimationState) :NewEnumerator0 "/Game/Player/Sprites/FlipBook/Idle.Idle" :NewEnumerator1 "/Game/Player/Sprites/FlipBook/Run.Run" :NewEnumerator2 "/Game/Player/Sprites/FlipBook/Jump.Jump" :NewEnumerator3 "/Game/Player/Sprites/FlipBook/Glide.Glide" :NewEnumerator4 "/Game/Player/Sprites/FlipBook/Attack.Attack" :NewEnumerator5 "/Game/Player/Sprites/FlipBook/Throw.Throw")))