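; BP_Tree is a Paper2D enemy that turns to face the player, creeps toward them along X and shoots at close range.
; Tick checks X distance to drive movement and firing, with a DoOnce and Delay throttling bullet spawns from an Arrow.
; It registers with the tagged GameController on BeginPlay for an ID-based name.
; Damage reduces health, and death notifies that controller before destroying the actor.
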(event Custom|DmgBadMan
  (params (DmgTaken :type Integer))
  ;[1 1 1] DmgToBadMan and death
  (bind _output_get (Variables|Default|SetbadMan_health (- (Variables|Default|GetbadMan_health) DmgTaken)))
  (if (<= _output_get 0)
    (bind _asgame_controller (Utilities|Casting|CastToGameController (Variables|Default|GetgameController)))
    (Default|EnemyDie _asgame_controller)
    (Development|PrintString (Variables|Default|Getname))
    (Actor|DestroyActor)
    (else
      (Development|PrintString (Utilities|String|ToString(Integer) (Variables|Default|GetbadMan_health))))))

(event Custom|BadMan_Shoot
  ;[1 1 1] Shoot
  (Utilities|FlowControl|DoOnce false :!label _label
    (:Completed
      (Game|SpawnActorfromClass "/Game/Enemy/badGuy_bullet.badGuy_bullet_C" (Transformation|GetWorldTransform (Variables|Default|GetArrow)) "Undefined" 0 0)
      (Utilities|FlowControl|Delay 0.75)
      (goto _label Reset))))

(event EventBeginPlay
  ;[1 1 1] EventBegin (GameControl info)
  (bind _outactors (Actor|GetAllActorswithTag "GameController"))
  (bind _output_get (Variables|Default|SetgameController (Utilities|Array|Get(acopy) _outactors)))
  (bind _asgame_controller (Utilities|Casting|CastToGameController _output_get))
  (Default|EnemySpawn _asgame_controller)
  (Variables|Default|Setname (Utilities|String|Append (Utilities|String|MakeLiteralString (Variables|Default|GetenemyType)) (Utilities|String|ToString(Integer) (Variables|/Game/GameController.GameController_C|GetenemyID _asgame_controller)))))

(event EventTick
  (params (DeltaSeconds :type Float%20%28single-precision%29))
  (bind _returnvalue (Transformation|GetActorLocation))
  ;[1 1 1] TargetAndShoot
  (Utilities|FlowControl|Sequence
    (:then_0
      (bind _output_get (Variables|Default|SetDistance (- (.x (Transformation|GetWorldLocation (Variables|Default|GetPaperFlipbook))) (.x (Transformation|GetActorLocation (Game|GetPlayerCharacter 0))))))
      (if (Math|Float|InRange(Float) _output_get -3e+02 3e+02)
        (CallFunction|BadManShoot)))
    (:then_1
      (Transformation|SetActorRotation (Math|Rotator|MakeRotator 0.0 0.0 (.yaw (Math|Rotator|FindLookatRotation (Transformation|GetActorLocation) (Transformation|GetActorLocation (Game|GetPlayerCharacter 0)))))))
    (:then_2
      (Variables|Default|SetActorX (.x _returnvalue)))
    (:then_3
      (Variables|Default|SetActorY (.y _returnvalue)))
    (:then_4
      (Variables|Default|SetActorZ (.z _returnvalue)))
    (:then_5
      (if (Math|Float|InRange(Float) (Variables|Default|GetDistance) 0.0 5e+02)
        (Utilities|FlowControl|Delay 0.01)
        (Transformation|SetActorLocation (Math|Vector|MakeVector (- (Variables|Default|GetActorX) 1.5) (Variables|Default|GetActorY) (Variables|Default|GetActorZ)) false false)))
    (:then_6
      (if (Math|Float|InRange(Float) (Variables|Default|GetDistance) -5e+02 0.0)
        (Utilities|FlowControl|Delay 0.01)
        (Transformation|SetActorLocation (Math|Vector|MakeVector (+ (Variables|Default|GetActorX) 1.5) (Variables|Default|GetActorY) (Variables|Default|GetActorZ)) false false)))))

(fn ConstructionScript)